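; Spotlight row actor that generates evenly spaced, downward-facing lights with optional random flicker.
; The construction script adds the spotlight components along local X around the origin at a set height, applies shared intensity, cone, attenuation and temperature settings, and stores them in an array.
; When flicker is enabled, BeginPlay starts a self-retriggering event loop that waits randomly, picks one light, pulses its intensity in a random-length burst, then restores it.
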(event Custom|FlickerBurst
  (bind _currentflickerlight (Variables|Default|GetCurrentFlickerLight))
  (Utilities|IsValid _currentflickerlight
    (:Is%20Valid
      (Rendering|Components|Light|SetIntensity _currentflickerlight (Variables|Default|GetFlickerOffIntensity))
      (Utilities|FlowControl|Delay (Math|Random|RandomFloatinRange (Variables|Default|GetFlickerOffTimeMin) (Variables|Default|GetFlickerOffTimeMax)))
      (Rendering|Components|Light|SetIntensity (Variables|Default|GetCurrentFlickerLight) (Variables|Default|GetFlickerOnIntensity))
      (Utilities|FlowControl|Delay (Math|Random|RandomFloatinRange (Variables|Default|GetFlickerOnTimeMin) (Variables|Default|GetFlickerOnTimeMax)))
      (bind _result (Math|Integer|DecrementInt (Variables|Default|GetRemainingFlickerCount))
        (:%20%20
          (bind _output_get (Variables|Default|SetRemainingFlickerCount _result))
          (if (> _output_get 0)
            (CallFunction|FlickerBurst)
            (else
              (Rendering|Components|Light|SetIntensity (Variables|Default|GetCurrentFlickerLight) (Variables|Default|GetLightIntensity))
              (CallFunction|StartRandomFlicker))))))))

(event Custom|StartRandomFlicker
  (Utilities|FlowControl|Delay (Math|Random|RandomFloatinRange (Variables|Default|GetFlickerDelayMin) (Variables|Default|GetFlickerDelayMax)))
  (Variables|Default|SetCurrentFlickerLight (Utilities|Array|Get(acopy) (Variables|Default|GetSpotLights) (Math|Random|RandomIntegerinRange 0 (- (Utilities|Array|Length (Variables|Default|GetSpotLights)) 1))))
  (Variables|Default|SetRemainingFlickerCount (Math|Random|RandomIntegerinRange (Variables|Default|GetFlickerBurstMin) (Variables|Default|GetFlickerBurstMax)))
  (CallFunction|FlickerBurst))

(event EventBeginPlay
  (if (Variables|Default|GetbUseFlicker)
    (CallFunction|StartRandomFlicker)))

(event Collision|EventActorBeginOverlap
  (params (OtherActor :type Actor%20Object%20Reference)))

(event EventTick
  (params (DeltaSeconds :type Float%20%28single-precision%29)))

(fn ConstructionScript
  (Utilities|Array|Clear (Variables|Default|GetSpotLights))
  (for _index (range 0 (Variables|Default|GetLightCount))
    (bind _returnvalue (AddComponent|AddSpotLightComponent false (Math|Transform|MakeTransform (Math|Vector|MakeVector (+ (* _index (Variables|Default|GetSpacing)) (* (* (* (Variables|Default|GetLightCount) (Variables|Default|GetSpacing)) 0.5) -1.0)) 0.0 (Variables|Default|GetHeight)) "-90.000000,0.000000,0.000000" "1.000000,1.000000,1.000000")))
    (Rendering|Components|Light|SetIntensity _returnvalue (Variables|Default|GetLightIntensity))
    (Rendering|Lighting|SetAttenuationRadius _returnvalue (Variables|Default|GetAttentionRadius))
    (Rendering|Lighting|SetInnerConeAngle _returnvalue (Variables|Default|GetInnerConeAngle))
    (Rendering|Lighting|SetOuterConeAngle _returnvalue (Variables|Default|GetOuterConeAngle))
    (Class|LightComponent|SetUseTemperature _returnvalue (Variables|Default|GetbUseTemperature))
    (Class|LightComponent|SetTemperature _returnvalue (Variables|Default|GetTemperature))
    (Utilities|Array|Add (Variables|Default|GetSpotLights) _returnvalue)))
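; BP_ImpactFloor is a floor that shatters once when a crash is triggered at an impact point.
; TriggerCrash, guarded by HasFractured, calls FractureFloor and then the CrashFloor dispatcher with the impact location and strength.
; FractureFloor swaps the static mesh for a simulating GCFloor that ignores Pawns and receives a radial impulse at that point.
; The impulse uses a fixed strength, independent of ImpactStrength.
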(event Custom|TriggerCrash
  (params (ImpactLocation :type Vector) (ImpactStrength :type Float%20%28double-precision%29))
  (if (not (Variables|Default|GetbHasFractured))
    (Variables|Default|SetbHasFractured true)
    (CallFunction|FractureFloor ImpactLocation)
    (Default|CallCrashFloor ImpactLocation ImpactStrength)))

(event EventBeginPlay)

(event Collision|EventActorBeginOverlap
  (params (OtherActor :type Actor%20Object%20Reference)))

(event EventTick
  (params (DeltaSeconds :type Float%20%28single-precision%29)))

(fn ConstructionScript)

(fn FractureFloor
  (params (Origin :type Vector))
  (bind _staticmeshcomponent (Variables|Debug|GetStaticMeshComponent))
  (bind _gc_floor (Variables|Default|GetGC_Floor))
  (Rendering|SetVisibility _staticmeshcomponent false false)
  (Collision|SetCollisionEnabled _staticmeshcomponent "NoCollision")
  (Rendering|SetVisibility _gc_floor true false)
  (Development|SetHiddeninGame _gc_floor false false)
  (Collision|SetCollisionEnabled _gc_floor "QueryAndPhysics")
  (Collision|SetCollisionResponsetoChannel _gc_floor "ECC_Pawn" "ECR_Ignore")
  (Physics|SetSimulatePhysics _gc_floor true)
  (Class|PrimitiveComponent|WakeRigidBody _gc_floor "None")
  (Physics|AddRadialImpulse _gc_floor Origin 1.5e+03 1.5e+03 "RIF_Linear" false))
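; BP_Room is a sci-fi bedroom room actor that marks both sides of its door for the Remy character.
; Two trigger volumes, OpenDoorInside and OpenDoorOutside, each set Remy's Open flag and store the opposite trigger's location as its TeleportPoint on overlap.
; Leaving either trigger clears Open, while any actual teleporting is left to Remy.
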(event OnComponentBeginOverlap(OpenDoorInside)
  (params (OverlappedComponent :type Primitive%20Component%20Object%20Reference) (OtherActor :type Actor%20Object%20Reference) (OtherComp :type Primitive%20Component%20Object%20Reference) (OtherBodyIndex :type Integer) (bFromSweep :type Boolean) (SweepResult :type Hit%20Result%20Structure%20%28by%20ref%29))
  (bind _asremy (Utilities|Casting|CastToRemy OtherActor))
  (Variables|/Game/Character/BluePrints/Remy.Remy_C|SetOpen? _asremy true)
  (Variables|/Game/Character/BluePrints/Remy.Remy_C|SetTeleportPoint _asremy (Transformation|GetWorldLocation (Variables|Default|GetOpenDoorOutside))))

(event OnComponentEndOverlap(OpenDoorInside)
  (params (OverlappedComponent :type Primitive%20Component%20Object%20Reference) (OtherActor :type Actor%20Object%20Reference) (OtherComp :type Primitive%20Component%20Object%20Reference) (OtherBodyIndex :type Integer))
  (bind _asremy (Utilities|Casting|CastToRemy OtherActor))
  (Variables|/Game/Character/BluePrints/Remy.Remy_C|SetOpen? _asremy false))

(event OnComponentBeginOverlap(OpenDoorOutside)
  (params (OverlappedComponent :type Primitive%20Component%20Object%20Reference) (OtherActor :type Actor%20Object%20Reference) (OtherComp :type Primitive%20Component%20Object%20Reference) (OtherBodyIndex :type Integer) (bFromSweep :type Boolean) (SweepResult :type Hit%20Result%20Structure%20%28by%20ref%29))
  (bind _asremy (Utilities|Casting|CastToRemy OtherActor))
  (Variables|/Game/Character/BluePrints/Remy.Remy_C|SetOpen? _asremy true)
  (Variables|/Game/Character/BluePrints/Remy.Remy_C|SetTeleportPoint _asremy (Transformation|GetWorldLocation (Variables|Default|GetOpenDoorInside))))

(event OnComponentEndOverlap(OpenDoorOutside)
  (params (OverlappedComponent :type Primitive%20Component%20Object%20Reference) (OtherActor :type Actor%20Object%20Reference) (OtherComp :type Primitive%20Component%20Object%20Reference) (OtherBodyIndex :type Integer))
  (bind _asremy (Utilities|Casting|CastToRemy OtherActor))
  (Variables|/Game/Character/BluePrints/Remy.Remy_C|SetOpen? _asremy false))

(event EventBeginPlay)

(event Collision|EventActorBeginOverlap
  (params (OtherActor :type Actor%20Object%20Reference)))

(event EventTick
  (params (DeltaSeconds :type Float%20%28single-precision%29)))

(fn ConstructionScript)
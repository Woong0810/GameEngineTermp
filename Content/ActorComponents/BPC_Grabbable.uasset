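; BPC_Grabbable is an actor component that tracks held state for a grabbable primitive and shows an outline mesh while held.
; InitializeTarget stores both references and hides the outline; BeginPlay calls it without arguments.
; Grab checks CanGrab, disables physics and shows any outline, leaving attachment undone and Holder unused.
; Release hides the outline, restores physics and clears IsHeld only when both target and outline are valid.
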(event EventBeginPlay
  (CallFunction|InitializeTarget))

(event EventTick
  (params (DeltaSeconds :type Float%20%28single-precision%29)))

(fn InitializeTarget
  (params (InTargetPrimitive :type Primitive%20Component%20Object%20Reference) (InOutlineMesh :type Static%20Mesh%20Component%20Object%20Reference))
  (Variables|Default|SetTargetPrimitive InTargetPrimitive)
  (bind _output_get (Variables|Default|SetOutlineMesh InOutlineMesh))
  (Utilities|IsValid _output_get
    (:Is%20Valid
      (Rendering|SetVisibility _output_get false false))))

(fn CanGrab
  (return (and (not (Variables|Default|GetbIsHeld)) (Utilities|IsValid (Variables|Default|GetTargetPrimitive)))))

(fn Grab
  (params (Holder :type Actor%20Object%20Reference))
  (bind _outlinemesh (Variables|Default|GetOutlineMesh))
  (bind _result (CallFunction|CanGrab))
  (if _result
    (Variables|Default|SetbIsHeld true)
    (Physics|SetSimulatePhysics (Variables|Default|GetTargetPrimitive) false)
    (Utilities|IsValid _outlinemesh
      (:Is%20Valid
        (Rendering|SetVisibility _outlinemesh true false)))))

(fn Release
  (bind _outlinemesh (Variables|Default|GetOutlineMesh))
  (Utilities|IsValid (Variables|Default|GetTargetPrimitive)
    (:Is%20Valid
      (Utilities|IsValid _outlinemesh
        (:Is%20Valid
          (Rendering|SetVisibility _outlinemesh false false)
          (Physics|SetSimulatePhysics (Variables|Default|GetTargetPrimitive) true)
          (Variables|Default|SetbIsHeld false))))))
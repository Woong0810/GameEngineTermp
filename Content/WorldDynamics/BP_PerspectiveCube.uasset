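; BP_PerspectiveCube is a grabbable cube actor that always reports it can be grabbed.
; At BeginPlay it hands its static mesh and outline mesh to the BPCGrabbable component, then forwards grab and release events to it.
; A drop camera shake, gated by impact normal, velocity and actor scale and strengthened with size, is present but disconnected, and the hit event is empty.
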(event OnComponentHit(StaticMeshComponent)
  (params (HitComponent :type Primitive%20Component%20Object%20Reference) (OtherActor :type Actor%20Object%20Reference) (OtherComp :type Primitive%20Component%20Object%20Reference) (NormalImpulse :type Vector :default "0, 0, 0") (Hit :type Hit%20Result%20Structure%20%28by%20ref%29)))

(event EventBeginPlay
  (Default|InitializeTarget (Variables|Default|GetBPC_Grabbable) (Variables|Debug|GetStaticMeshComponent) (Variables|Default|GetOutlineMesh)))

(event Collision|EventActorBeginOverlap
  (params (OtherActor :type Actor%20Object%20Reference)))

(event EventTick
  (params (DeltaSeconds :type Float%20%28single-precision%29)))

(event EventGrabObject
  (params (Holder :type Actor%20Object%20Reference))
  (Default|Grab (Variables|Default|GetBPC_Grabbable) Holder))

(event EventReleaseGrab
  (params (Holder :type Actor%20Object%20Reference))
  (Default|Release (Variables|Default|GetBPC_Grabbable)))

(fn ConstructionScript)

(fn CanGrab
  (return true))
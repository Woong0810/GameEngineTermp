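; BP_PerspectiveObject is a grabbable physical prop whose impact feedback depends on its actor scale.
; Grab, release and CanGrab calls forward to BPCGrabbable, set up on BeginPlay with the mesh and outline.
; Fast hits on upward-facing non-player surfaces play a throttled soft sound when small, or a heavy sound and scale-driven camera shake when large.
; Heavy hits can fracture BP_ImpactFloor; grabbing re-arms this one-shot impact response.
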(event OnComponentHit(StaticMeshComponent)
  (params (HitComponent :type Primitive%20Component%20Object%20Reference) (OtherActor :type Actor%20Object%20Reference) (OtherComp :type Primitive%20Component%20Object%20Reference) (NormalImpulse :type Vector :default "0, 0, 0") (Hit :type Hit%20Result%20Structure%20%28by%20ref%29))
  (bind _returnvalue (Transformation|GetActorScale3D))
  (bind (_bblockinghit _binitialoverlap _time _distance _location _impactpoint _normal _impactnormal) (Collision|BreakHitResult Hit))
  (bind _staticmeshcomponent (Variables|Debug|GetStaticMeshComponent))
  (bind _returnvalue_2 (Transformation|GetComponentVelocity _staticmeshcomponent))
  (bind _returnvalue_3 (Math|Vector|VectorLength _returnvalue_2))
  (if (Variables|Default|GetbCanHeavyDropShake)
    (if (!= OtherActor (Game|GetPlayerCharacter 0))
      (if (> (.z _impactnormal) 0.7)
        (if (> (Math|Vector|VectorLength (Transformation|GetComponentVelocity (Variables|Debug|GetStaticMeshComponent))) (Variables|Default|GetShakeVelocity))
          (if (> (.x _returnvalue) (Variables|Default|GetShakeScale))
            (Utilities|FlowControl|Sequence
              (:then_0
                (Audio|PlaySoundatLocation "/Game/Audios/HeavyDrop.HeavyDrop" _impactpoint "0, 0, 0" 0.5 1.0 0.0 0 0 0 0)
                (CameraShakes|StartCameraShake (Game|GetPlayerCameraManager 0) "/Game/BluePrints/BP_HeavyDropShake.BP_HeavyDropShake_C" (Math|Float|MapRangeClamped (.x _returnvalue) 1.0 5.0 1.0 5.0) "CameraLocal" "0, 0, 0")
                (Variables|Default|SetbCanHeavyDropShake false))
              (:then_1
                (bind _asbp_impact_floor (Utilities|Casting|CastToBP_ImpactFloor OtherActor))
                (if (> _returnvalue_3 (Variables|Default|GetFractureVelocity))
                  (if (> (.x (Transformation|GetActorScale3D)) (Variables|Default|GetFractureScale))
                    (Default|TriggerCrash _asbp_impact_floor _impactpoint _returnvalue_3)))))
            (elif (Variables|Default|GetbCanPlayDropSound)
              (Variables|Default|SetbCanPlayDropSound false)
              (Audio|PlaySoundatLocation "/Game/Audios/SoftDrop.SoftDrop" "0, 0, 0" "0, 0, 0" 0.5 1.0 0.0 0 0 0 0)
              (Utilities|FlowControl|Delay 0.7)
              (Variables|Default|SetbCanPlayDropSound true))))))))

(event EventBeginPlay
  (Default|InitializeTarget (Variables|Default|GetBPC_Grabbable) (Variables|Debug|GetStaticMeshComponent) (Variables|Default|GetOutlineMesh)))

(event Collision|EventActorBeginOverlap
  (params (OtherActor :type Actor%20Object%20Reference)))

(event EventTick
  (params (DeltaSeconds :type Float%20%28single-precision%29)))

(event EventGrabObject
  (params (Holder :type Actor%20Object%20Reference))
  (Default|Grab (Variables|Default|GetBPC_Grabbable) Holder)
  (Variables|Default|SetbCanHeavyDropShake true))

(event EventReleaseGrab
  (params (Holder :type Actor%20Object%20Reference))
  (Default|Release (Variables|Default|GetBPC_Grabbable)))

(fn ConstructionScript)

(fn CanGrab
  (bind _result (Default|CanGrab (Variables|Default|GetBPC_Grabbable)))
  (return _result))